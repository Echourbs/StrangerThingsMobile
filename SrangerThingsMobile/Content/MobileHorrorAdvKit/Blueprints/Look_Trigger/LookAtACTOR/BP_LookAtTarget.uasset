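; Trigger actor that turns the player's view toward a sequence of target actors when the MobileHorrorKitCharacter overlaps its box.
; A timeline lerps the controller's rotation from the current eye rotation toward each LookTarget along the shortest path.
; When it finishes, CheckTargetsOrder advances the index, waits that entry's LookingTime and replays the look, resetting the index after the last target.
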(event OnComponentBeginOverlap(Box)
  (params (OverlappedComponent :type Primitive%20Component%20Object%20Reference) (OtherActor :type Actor%20Object%20Reference) (OtherComp :type Primitive%20Component%20Object%20Reference) (OtherBodyIndex :type Integer) (bFromSweep :type Boolean) (SweepResult :type Hit%20Result%20Structure%20%28by%20ref%29))
  (bind _returnvalue (Game|GetPlayerCharacter 0))
  ;[0.3087 0.776 0.5235] Look At Target Settings
  (bind _asmobile_horror_kit_character (Utilities|Casting|CastToMobileHorrorKitCharacter OtherActor))
  (Variables|Default|SetPlayer%20Reference _asmobile_horror_kit_character)
  (bind _newtrack_0 (Timeline|Timeline_0 PlayFromStart)
    (:Update
      (bind _output_get (Variables|Default|SetDefault%20Timeline _newtrack_0))
      (Pawn|SetControlRotation (Game|GetPlayerController 0) (Math|Rotator|Lerp(Rotator) (.OutRotation (Actor|GetActorEyesViewPoint _returnvalue)) (Math|Rotator|FindLookatRotation (Transformation|GetActorLocation _returnvalue) (Transformation|GetWorldLocation (Variables|/Script/Engine.Actor|GetRootComponent (Utilities|Array|Get(acopy) (Variables|Default|GetLookTarget) (Variables|Default|GetIndex))))) _output_get true)))
    (:Finished
      (Variables|Default|SetIndex (stale Custom|Check%20Targets%20Order _output_get))
      (CallFunction|CheckTargetsOrder))))

(event Custom|Look%20at%20Target
  (bind _returnvalue (Game|GetPlayerCharacter 0))
  ;[0.3087 0.776 0.5235] Look At Target Settings
  (bind _asmobile_horror_kit_character (Utilities|Casting|CastToMobileHorrorKitCharacter (stale OnComponentBeginOverlap(Box) OtherActor)))
  (Variables|Default|SetPlayer%20Reference _asmobile_horror_kit_character)
  (bind _newtrack_0 (Timeline|Timeline_0 PlayFromStart)
    (:Update
      (bind _output_get (Variables|Default|SetDefault%20Timeline _newtrack_0))
      (Pawn|SetControlRotation (Game|GetPlayerController 0) (Math|Rotator|Lerp(Rotator) (.OutRotation (Actor|GetActorEyesViewPoint _returnvalue)) (Math|Rotator|FindLookatRotation (Transformation|GetActorLocation _returnvalue) (Transformation|GetWorldLocation (Variables|/Script/Engine.Actor|GetRootComponent (Utilities|Array|Get(acopy) (Variables|Default|GetLookTarget) (Variables|Default|GetIndex))))) _output_get true)))
    (:Finished
      (Variables|Default|SetIndex (stale Custom|Check%20Targets%20Order _output_get))
      (CallFunction|CheckTargetsOrder))))

(event Custom|Check%20Targets%20Order
  ;[0.4635 0.2608 0.1755] Check Targets Order
  (if (>= (Variables|Default|GetIndex) (- (Utilities|Array|Length (Variables|Default|GetLookTarget)) 1))
    (bind _output_get (Variables|Default|SetIndex 0))
    (else
      (Math|Integer|IncrementInt (Variables|Default|GetIndex)
        (:%20%20
          (Utilities|FlowControl|Delay (Utilities|Array|Get(acopy) (Variables|Default|GetLooking%20Time) (Variables|Default|GetIndex)))
          (CallFunction|LookatTarget))))))

(fn ConstructionScript)